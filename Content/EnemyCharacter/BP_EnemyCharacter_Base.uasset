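; Base enemy character Blueprint that handles the death dissolve effect.
; On death it pauses animation, disables capsule collision, and runs a timeline scaled by TotalDissolveTime that drives DissolveAmount on the mesh and equipped weapon materials.
; It async-loads and attaches a Niagara system, tinting its particles with the mesh material's DissolveEdgeColor.
; When the timeline finishes, it destroys the weapon and the character.
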(event EventBeginPlay)

(event Collision|EventActorBeginOverlap
  (params (OtherActor :type Actor%20Object%20Reference)))

(event EventTick
  (params (DeltaSeconds :type Float%20%28single-precision%29)))

(event EventOnEnemyDied
  (params (DissolveNiagaraSystem :type Niagara%20System%20Soft%20Object%20Reference))
  (Utilities|FlowControl|Sequence
    (:then_0
      (Variables|/Script/Engine.SkeletalMeshComponent|SetbPauseAnims (Variables|Character|GetMesh) true)
      (Collision|SetCollisionEnabled (Variables|Default|GetCapsuleComponent) "NoCollision"))
    (:then_1
      (|PlayDissolveMaterialAndDestroy))
    (:then_2
      (|AttachNiagaraSystem DissolveNiagaraSystem))))

(fn ConstructionScript)